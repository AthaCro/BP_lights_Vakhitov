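; BP_lights is a light Blueprint that blinks its SpotLight a limited number of times when play begins.
; A looping DoN gate runs five cycles, switching visibility to the LightOff and LightOn variables after alternating short delays.
; Each cycle also prints a FlipFlop state for debugging.
; Both branches have constant true conditions, so the paths that clear the SpotLight reference never run.
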(event `self.ReceiveBeginPlay`
  (`/Engine/EditorBlueprintResources/StandardMacros.Do N` 5 :!label _label
    (:`Exit`
      (bind _isa (`/Engine/EditorBlueprintResources/StandardMacros.FlipFlop`)
        (:`A`
          _)
        (:`B`
          _))
      (`KismetSystemLibrary.PrintString` (`KismetStringLibrary.Conv_BoolToString` _isa))
      (`KismetSystemLibrary.Delay` 0.5)
      (if true
        (`SceneComponent.SetVisibility` (`self.SpotLight`) (`self.LightOff`) false)
        (else
          (set `self.SpotLight` null)))
      (`KismetSystemLibrary.Delay` 1.0)
      (if true
        (`SceneComponent.SetVisibility` (`self.SpotLight`) (`self.lightOn`) false)
        (goto _label)
        (else
          (set `self.SpotLight` null)
          (goto _label))))))

(fn `UserConstructionScript`)